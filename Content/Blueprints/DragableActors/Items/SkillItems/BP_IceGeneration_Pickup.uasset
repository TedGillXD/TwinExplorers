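; Interactable pickup for the Ice Generation skill item.
; It swaps the skeletal mesh material between focused and unfocused variants when focus changes.
; It always allows interaction and builds its prompt from "拾取" (pick up) plus the item name in ItemData.
; The prompt icon is always the keyboard F key, as the input-device-based icon selection is left unconnected.
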(event `self.ReceiveBeginPlay`)

(event `InteractableInterface.Unfocused`
  (`PrimitiveComponent.SetMaterial` (`self.SkeletalMesh`) 0 (`self.UnfocusedMaterial`)))

(event `InteractableInterface.Focused`
  (`PrimitiveComponent.SetMaterial` (`self.SkeletalMesh`) 0 (`self.FocusedMaterial`)))

(fn `CanInteract`
  (params (InHandItem :type "Item Structure (by ref)"))
  (returns (ReturnValue :type Boolean))
  (return true))

(fn `GetInteractIcon`
  (returns (ReturnValue :type "Texture2D Object Reference"))
  (return "/Game/Textures/Keys/keyboard_f.keyboard_f"))

(fn `GetInteractString`
  (returns (ReturnValue :type String))
  (bind _itemdata_itemname (break `Item` (`self.ItemData`)))
  (return (`KismetStringLibrary.Concat_StrStr` "拾取 " (`KismetStringLibrary.Conv_NameToString` _itemdata_itemname))))

(fn `UserConstructionScript`)