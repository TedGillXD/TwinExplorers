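; BP_Door is a contraption door that moves on Activate and Deactivate events, driven by physics rather than animation.
; Activate enables physics on the Door, wakes it and sets the PhysicsConstraint linear position target to an offset along Z.
; Deactivate resets the target to zero, wakes the body and uses a short timer to switch physics simulation off again.
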(event `self.Activate`
  (`PrimitiveComponent.SetSimulatePhysics` (`self.Door`) true)
  (`PrimitiveComponent.WakeRigidBody` (`self.Door`) "None")
  (`PhysicsConstraintComponent.SetLinearPositionTarget` (`self.PhysicsConstraint`) (`KismetMathLibrary.MakeVector_NetQuantize` 0.0 0.0 -150.0)))

(event `self.Deactivate`
  (`PhysicsConstraintComponent.SetLinearPositionTarget` (`self.PhysicsConstraint`) (`KismetMathLibrary.MakeVector_NetQuantize` 0.0))
  (`PrimitiveComponent.WakeRigidBody` (`self.Door`) "None")
  (`KismetSystemLibrary.K2_SetTimerDelegate` (delegate `SetDoorSimulatePhysics`) 0.2))

(event `SetDoorSimulatePhysics`
  (`PrimitiveComponent.SetSimulatePhysics` (`self.Door`) false))

(fn `UserConstructionScript`)