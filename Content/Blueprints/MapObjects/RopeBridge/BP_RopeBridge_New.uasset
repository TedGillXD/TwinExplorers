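; Rope bridge map object made of eighteen individual plank components.
; On BeginPlay an authority check turns off physics simulation on every plank for remote (non-authority) instances, leaving the authority's planks untouched.
; The construction script and overlap event are empty, so this network-role switch is the only graph logic.
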(event `self.ReceiveBeginPlay`
  (`/Engine/EditorBlueprintResources/ActorMacros.Switch Has Authority`
    (:`Remote`
      (`PrimitiveComponent.SetSimulatePhysics` (`self.Plank6`) false)
      (`PrimitiveComponent.SetSimulatePhysics` (`self.Plank7`) false)
      (`PrimitiveComponent.SetSimulatePhysics` (`self.Plank8`) false)
      (`PrimitiveComponent.SetSimulatePhysics` (`self.Plank9`) false)
      (`PrimitiveComponent.SetSimulatePhysics` (`self.Plank10`) false)
      (`PrimitiveComponent.SetSimulatePhysics` (`self.Plank5`) false)
      (`PrimitiveComponent.SetSimulatePhysics` (`self.Plank1`) false)
      (`PrimitiveComponent.SetSimulatePhysics` (`self.Plank2`) false)
      (`PrimitiveComponent.SetSimulatePhysics` (`self.Plank15`) false)
      (`PrimitiveComponent.SetSimulatePhysics` (`self.Plank4`) false)
      (`PrimitiveComponent.SetSimulatePhysics` (`self.Plank11`) false)
      (`PrimitiveComponent.SetSimulatePhysics` (`self.Plank17`) false)
      (`PrimitiveComponent.SetSimulatePhysics` (`self.Plank18`) false)
      (`PrimitiveComponent.SetSimulatePhysics` (`self.Plank3`) false)
      (`PrimitiveComponent.SetSimulatePhysics` (`self.Plank14`) false)
      (`PrimitiveComponent.SetSimulatePhysics` (`self.Plank13`) false)
      (`PrimitiveComponent.SetSimulatePhysics` (`self.Plank12`) false)
      (`PrimitiveComponent.SetSimulatePhysics` (`self.Plank16`) false))))

(fn `UserConstructionScript`)