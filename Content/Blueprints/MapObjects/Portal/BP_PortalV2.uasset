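; BP_PortalV2 is a portal map object that grows into view and renders through a scene capture camera.
; On non-authority instances, BeginPlay shrinks the actor and plays the PortalScale timeline into CurrentScale, which Tick applies as uniform actor scale while below full size.
; Tick also calls CaptureScene on PortalCamera every frame, with or without authority.
; The file contains no active overlap or teleport logic.
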(event `self.ReceiveBeginPlay`
  (`|ExecutionSequence`
    (:`then_0`
      (`/Engine/EditorBlueprintResources/ActorMacros.Switch Has Authority`
        (:`Remote`
          (`self.SetActorScale3D` (0.1 0.1 0.1))
          (bind (_direction _newtrack_0) (`Timeline|PortalScale`)
            (:`Update`
              (set `self.CurrentScale` _newtrack_0))))))))

(event `self.ReceiveTick`
  (params (DeltaSeconds :type "Float (single-precision)"))
  (bind _currentscale (`self.CurrentScale`))
  (`|ExecutionSequence`
    (:`then_0`
      (`/Engine/EditorBlueprintResources/ActorMacros.Switch Has Authority`
        (:`Remote`
          (if (< (`self.CurrentScale`) 1.0)
            (`self.SetActorScale3D` (`KismetMathLibrary.MakeVector` _currentscale _currentscale _currentscale))))))
    (:`then_1`
      (`SceneCaptureComponent2D.CaptureScene` (`self.PortalCamera`)))))

(fn `UserConstructionScript`)