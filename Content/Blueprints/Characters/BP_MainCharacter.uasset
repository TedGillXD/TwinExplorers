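; Main player character Blueprint that handles networked overhead name display and portal skill input.
; On BeginPlay, remote instances load the saved name from the Setting slot and send it to the server.
; The server relays it to clients, passes existing GameState name mappings to SetAllPlayersName, then records the new entry.
; Portal inputs play sped-up shoot montages, while cancel deactivates the in-hand child actor's Skill.
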(event `SetNameOnAllClient`
  (params (Name :type String))
  ;[1 1 1] 设置角色姓名
  (bind _aswidget_character_name (cast `/Game/Blueprints/Widgets/Widget_CharacterName` (`WidgetComponent.GetWidget` (`self.CharacterNameWidget`))))
  (`/Game/Blueprints/Widgets/Widget_CharacterName.SetCharacterName` _aswidget_character_name Name))

(event `SetNameOnServer`
  (params (CharacterName :type String))
  ;[1 1 1] 设置角色姓名
  (`self.SetNameOnAllClient` CharacterName)
  (bind _asbp_main_level_game_state (cast `/Game/Blueprints/GameStates/BP_MainLevelGameState` (`GameplayStatics.GetGameState`)))
  (bind _namemapping (`MainLevelGameState.NameMapping` _asbp_main_level_game_state))
  (bind (_outcontrollers _outnames) (`NetworkFunctionLibrary.GetKeysAndValuesArrayFromMap` _namemapping))
  (`self.SetAllPlayersName` _outcontrollers _outnames)
  (`BlueprintMapLibrary.Map_Add` _namemapping self CharacterName))

(event `self.ReceiveBeginPlay`
  (`/Engine/EditorBlueprintResources/ActorMacros.Switch Has Authority`
    (:`Remote`
      (bind _returnvalue (`GameplayStatics.LoadGameFromSlot` "Setting"))
      (bind _assetting_save_game (cast `SettingSaveGame` _returnvalue))
      (`self.SetNameOnServer` (`SettingSaveGame.CharacterName` _assetting_save_game)))))

(event `EnhancedInput|/Game/Input/Actions/Portal/IA_Portal1`
  (params (ActionValue :type Boolean) (ElapsedSeconds :type "Float (double-precision)") (TriggeredSeconds :type "Float (double-precision)") (InputAction :type "InputAction Object Reference" :default "/Game/Input/Actions/Portal/IA_Portal1.IA_Portal1"))
  ;[1 1 1] Handle Portal Inputs
  (:`Triggered`
    (`self.PlayAnimMontage` "/Game/Animations/ShootPortal1_Montage.ShootPortal1_Montage" 3.0)))

(event `EnhancedInput|/Game/Input/Actions/Portal/IA_Portal2`
  (params (ActionValue :type Boolean) (ElapsedSeconds :type "Float (double-precision)") (TriggeredSeconds :type "Float (double-precision)") (InputAction :type "InputAction Object Reference" :default "/Game/Input/Actions/Portal/IA_Portal2.IA_Portal2"))
  ;[1 1 1] Handle Portal Inputs
  (:`Triggered`
    (`self.PlayAnimMontage` "/Game/Animations/ShootPortal2_Montage.ShootPortal2_Montage" 3.0)))

(event `EnhancedInput|/Game/Input/Actions/Portal/IA_PortalCancel`
  (params (ActionValue :type Boolean) (ElapsedSeconds :type "Float (double-precision)") (TriggeredSeconds :type "Float (double-precision)") (InputAction :type "InputAction Object Reference" :default "/Game/Input/Actions/Portal/IA_PortalCancel.IA_PortalCancel"))
  (bind _childactor (`ChildActorComponent.ChildActor` (`self.InHandItemActor`)))
  ;[1 1 1] Handle Portal Inputs
  (:`Triggered`
    (`/Engine/EditorBlueprintResources/StandardMacros.IsValid` _childactor
      (:`Is Valid`
        (bind _asskill (cast `Skill` _childactor))
        (`Skill.DeactivateSkill` _asskill self)))))

(event `self.SetCharacterName`
  (params (Name :type String))
  (bind _aswidget_character_name (cast `/Game/Blueprints/Widgets/Widget_CharacterName` (`WidgetComponent.GetWidget` (`self.CharacterNameWidget`))))
  (`/Game/Blueprints/Widgets/Widget_CharacterName.SetCharacterName` _aswidget_character_name Name))

(fn `UserConstructionScript`)