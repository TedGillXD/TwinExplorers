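; BP_GravityGun is the gravity gun item, exposed as an interactable pickup; it contains no gravity or firing logic.
; CanInteract always allows interaction, and GetInteractString builds the prompt from "拾取" (pick up) plus the item name in ItemData.
; GetInteractIcon casts the owner to a Character, then branches on its BP_MainCharacterController's keyboard or gamepad input, though no branch shows an icon value.
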(event `self.ReceiveBeginPlay`)

(fn `CanInteract`
  (params (InHandItem :type "Item Structure (by ref)"))
  (returns (ReturnValue :type Boolean))
  (return true))

(fn `GetInteractIcon`
  (params (InHandItem :type "Item Structure (by ref)"))
  (returns (ReturnValue :type "Texture2D Object Reference"))
  (bind _ascharacter (cast `Character` (`self.GetOwner`))
    (:`then`
      (bind _asbp_main_character_controller (cast `/Game/Blueprints/Controllers/BP_MainCharacterController` (`Pawn.GetController` _ascharacter))
        (:`then`
          (switch `EInputDevice` (`TEPlayerController.GetCurrentInputDevice` _asbp_main_character_controller)
            (:`Keyboard`
              (return null))
            (:`GamePad`
              (return null))))
        (:`CastFailed`
          (return null))))
    (:`CastFailed`
      (return null))))

(fn `GetInteractString`
  (params (InHandItem :type "Item Structure (by ref)"))
  (returns (ReturnValue :type String))
  (bind _itemdata_itemname (break `Item` (`self.ItemData`)))
  (return (`KismetStringLibrary.Concat_StrStr` "拾取 " (`KismetStringLibrary.Conv_NameToString` _itemdata_itemname))))

(fn `UserConstructionScript`)