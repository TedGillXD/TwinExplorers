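; Portal generation skill actor that lets a character shoot two portals through its PortalGenerationComponent.
; Activation enables input on the owner's TEPlayerController, adds the skill's Enhanced Input mapping context and resets the component.
; Each portal action fires its shot and uses the in-hand inventory item.
; The cancel action triggers deactivation, which disables input and removes the mapping context.
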(event `self.ActivateSkill`
  (params (CharacterBase :type "MainCharacterBase Object Reference"))
  (bind _output_get (set `self.InvokeCharacter` CharacterBase))
  (bind _asteplayer_controller (cast `TEPlayerController` (`Pawn.GetController` _output_get)))
  (bind _output_get_2 (set `self.As TEPlayer Controller` _asteplayer_controller))
  (`self.EnableInput` _output_get_2)
  (`EnhancedInputSubsystemInterface.AddMappingContext` (pcsubsystem `EnhancedInputLocalPlayerSubsystem` _output_get_2) (`self.SkillIMC`) 0 (struct))
  (`PortalGenerationComponent.Reset` (`MainCharacterBase.PortalGenerationComponent` (`self.InvokeCharacter`))))

(event `self.DeactivateSkill`
  (params (CharacterBase :type "MainCharacterBase Object Reference"))
  (`self.DisableInput` (`self.As TEPlayer Controller`))
  (`EnhancedInputSubsystemInterface.RemoveMappingContext` (pcsubsystem `EnhancedInputLocalPlayerSubsystem` (`self.As TEPlayer Controller`)) (`self.SkillIMC`) (struct)))

(event `EnhancedInput|/Game/Input/Actions/Portal/IA_Portal1`
  (params (ActionValue :type Boolean) (ElapsedSeconds :type "Float (double-precision)") (TriggeredSeconds :type "Float (double-precision)") (InputAction :type "InputAction Object Reference" :default "/Game/Input/Actions/Portal/IA_Portal1.IA_Portal1"))
  (:`Triggered`
    (`PortalGenerationComponent.ShootPortal1` (`MainCharacterBase.PortalGenerationComponent` (`self.InvokeCharacter`)))
    (`InventoryComponent.UseInHandItem` (`MainCharacterBase.InventoryComponent` (`self.InvokeCharacter`)))))

(event `EnhancedInput|/Game/Input/Actions/Portal/IA_Portal2`
  (params (ActionValue :type Boolean) (ElapsedSeconds :type "Float (double-precision)") (TriggeredSeconds :type "Float (double-precision)") (InputAction :type "InputAction Object Reference" :default "/Game/Input/Actions/Portal/IA_Portal2.IA_Portal2"))
  (:`Triggered`
    (`PortalGenerationComponent.ShootPortal2` (`MainCharacterBase.PortalGenerationComponent` (`self.InvokeCharacter`)))
    (`InventoryComponent.UseInHandItem` (`MainCharacterBase.InventoryComponent` (`self.InvokeCharacter`)))))

(event `EnhancedInput|/Game/Input/Actions/Portal/IA_PortalCancel`
  (params (ActionValue :type Boolean) (ElapsedSeconds :type "Float (double-precision)") (TriggeredSeconds :type "Float (double-precision)") (InputAction :type "InputAction Object Reference" :default "/Game/Input/Actions/Portal/IA_PortalCancel.IA_PortalCancel"))
  (:`Triggered`
    (`self.DeactivateSkill` (`self.InvokeCharacter`))))

(fn `UserConstructionScript`)