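; BP_IceGen_Skill is the ice pillar generation skill, with activate, generate and cancel handling.
; Activation starts the character's IceGenerationComponent spawn check, adds the skill's input mapping context and enables input on itself.
; Generate plays the shoot montage on all clients with a 2D sound, leaving the spawn outside this graph.
; Cancel runs deactivation, which disables input, cancels the check and calls FinishSpawningIcePillar on the character.
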(event `self.ActivateSkill`
  (params (CharacterBase :type "MainCharacterBase Object Reference"))
  (`IceGenerationComponent.DoSpawnCheck` (`MainCharacterBase.IceGenerationComponent` CharacterBase))
  (bind _asteplayer_controller (cast `TEPlayerController` (`Pawn.GetController` CharacterBase)))
  (`EnhancedInputSubsystemInterface.AddMappingContext` (pcsubsystem `EnhancedInputLocalPlayerSubsystem` _asteplayer_controller) (`self.SkillIMC`) 1 (struct))
  (set `self.InvokeCharacter` CharacterBase)
  (bind _output_get (set `self.InvokeController` _asteplayer_controller))
  (`self.EnableInput` _output_get))

(event `self.DeactivateSkill`
  (params (CharacterBase :type "MainCharacterBase Object Reference"))
  (bind _asteplayer_controller (cast `TEPlayerController` (`Pawn.GetController` CharacterBase)))
  (`self.DisableInput` _asteplayer_controller)
  (`IceGenerationComponent.CancelCheck` (`MainCharacterBase.IceGenerationComponent` CharacterBase))
  (`MainCharacterBase.FinishSpawningIcePillar` CharacterBase (`self.SkillIMC`)))

(event `EnhancedInput|/Game/Input/Actions/GenerateIce/IA_Generate`
  (params (ActionValue :type Boolean) (ElapsedSeconds :type "Float (double-precision)") (TriggeredSeconds :type "Float (double-precision)") (InputAction :type "InputAction Object Reference" :default "/Game/Input/Actions/GenerateIce/IA_Generate.IA_Generate"))
  (:`Triggered`
    (`MainCharacterBase.PlayMontageOnAllClient` (`self.InvokeCharacter`) "/Game/Animations/ShootIcePillar_Montage.ShootIcePillar_Montage" 3.0)
    (`GameplayStatics.PlaySound2D` "/Game/Sounds/Effects/Shot_Cue.Shot_Cue" 1.0 1.0 0.0 null null)))

(event `EnhancedInput|/Game/Input/Actions/GenerateIce/IA_Cancel`
  (params (ActionValue :type Boolean) (ElapsedSeconds :type "Float (double-precision)") (TriggeredSeconds :type "Float (double-precision)") (InputAction :type "InputAction Object Reference" :default "/Game/Input/Actions/GenerateIce/IA_Cancel.IA_Cancel"))
  (:`Triggered`
    (`self.DeactivateSkill` (`self.InvokeCharacter`))))

(fn `UserConstructionScript`)