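; BP_SpeedUp_Skill is a skill Blueprint that gives a character a temporary walk speed boost and uses up the in-hand item.
; ActivateSkill caches the character's current max speed, raises MaxWalkSpeed by a fixed multiplier and calls UseInHandItem on the invoking character's inventory.
; A one-shot timer lasting SkillLastTime then fires Recover to restore the cached speed, while DeactivateSkill is left empty.
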(event `self.ActivateSkill`
  (params (CharacterBase :type "MainCharacterBase Object Reference"))
  (bind _charactermovement (`Character.CharacterMovement` CharacterBase))
  (set `self.Character Base` CharacterBase)
  (bind _output_get (set `self.OriginalSpeed` (`MovementComponent.GetMaxSpeed` _charactermovement)))
  (set `CharacterMovementComponent.MaxWalkSpeed` (* _output_get 1.2) _charactermovement)
  (`InventoryComponent.UseInHandItem` (`MainCharacterBase.InventoryComponent` (`self.InvokeCharacter`)))
  (`KismetSystemLibrary.K2_SetTimerDelegate` (delegate `Recover`) (`self.SkillLastTime`)))

(event `self.DeactivateSkill`
  (params (CharacterBase :type "MainCharacterBase Object Reference")))

(event `Recover`
  (set `CharacterMovementComponent.MaxWalkSpeed` (`self.OriginalSpeed`) (`Character.CharacterMovement` (`self.Character Base`))))

(fn `UserConstructionScript`)